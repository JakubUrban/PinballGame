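; BP_Plunger is a plunger actor, apparently a pinball-style launcher, that pulls back while charging and snaps back on release.
; ChargePlunger runs a timeline that lerps the Plunger component along its local Y axis without sweeping.
; ReleasePlunger stops the timeline and quickly returns the component to rest with MoveComponentTo.
; GetBallSpawnLocation converts the local BallSpawnLocation to world space using the actor transform.
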(event Custom|ChargePlunger
  (bind _chargingplumbertrack (Timeline|ChargingPlungerTimeline PlayFromStart)
    (:Update
      (Transformation|SetRelativeLocation (Variables|Default|GetPlunger) (Math|Vector|Lerp(Vector) "0, 0, 0" "0,150.000000,0.000000" _chargingplumbertrack) false false))))

(event Custom|ReleasePlunger
  (Utilities|FlowControl|Sequence
    (:then_0
      (bind _chargingplumbertrack (Timeline|ChargingPlungerTimeline Stop)
        (:Update
          (Transformation|SetRelativeLocation (Variables|Default|GetPlunger) (Math|Vector|Lerp(Vector) "0, 0, 0" "0,150.000000,0.000000" _chargingplumbertrack) false false))))
    (:then_1
      (Components|MoveComponentTo (Variables|Default|GetPlunger) "0, 0, 0" "0, 0, 0" false false 0.14 false))))

(event EventBeginPlay)

(event Collision|EventActorBeginOverlap
  (params (OtherActor :type Actor%20Object%20Reference)))

(event EventTick
  (params (DeltaSeconds :type Float%20%28single-precision%29)))

(fn ConstructionScript)

(fn GetBallSpawnLocation
  (return (Math|Transform|TransformLocation (Transformation|GetActorTransform) (Variables|Default|GetBallSpawnLocation))))