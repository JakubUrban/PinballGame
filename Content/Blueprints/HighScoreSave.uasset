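; HighScoreSave holds the game's high score table as an array of score structs in SaveStruct.
; AddHighScore appends a new entry, re-sorts the table from highest to lowest and trims it to at most four entries.
; The sort is a selection sort that repeatedly moves the DetermineHighestScoreValue result into a temporary array.
; DetermineLowestScoreValue returns the lowest entry and its index, but nothing in this file calls it.
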(fn DetermineLowestScoreValue
  (for (_array_element _array_index) (Variables|Default|GetSaveStruct)
    (if (== _array_index 0)
      (LocalVariables|SetLowestScoreValue (.Score (Utilities|Struct|BreakHighScoreStruct _array_element)))
      (LocalVariables|SetLowestScoreIndex _array_index)
      (elif (< (.Score (Utilities|Struct|BreakHighScoreStruct _array_element)) (LocalVariables|GetLowestScoreValue))
        (LocalVariables|SetLowestScoreValue (.Score (Utilities|Struct|BreakHighScoreStruct _array_element)))
        (LocalVariables|SetLowestScoreIndex _array_index))))
  (return (Utilities|Array|Get(acopy) (Variables|Default|GetSaveStruct) (LocalVariables|GetLowestScoreIndex)) (LocalVariables|GetLowestScoreIndex)))

(fn DetermineHighestScoreValue
  (for (_array_element _array_index) (Variables|Default|GetSaveStruct)
    (if (== _array_index 0)
      (LocalVariables|SetHighestScoreValue (.Score (Utilities|Struct|BreakHighScoreStruct _array_element)))
      (LocalVariables|SetHighestScoreIndex _array_index)
      (elif (> (.Score (Utilities|Struct|BreakHighScoreStruct _array_element)) (LocalVariables|GetHighestScoreValue))
        (LocalVariables|SetHighestScoreValue (.Score (Utilities|Struct|BreakHighScoreStruct _array_element)))
        (LocalVariables|SetHighestScoreIndex _array_index))))
  (return (Utilities|Array|Get(acopy) (Variables|Default|GetSaveStruct) (LocalVariables|GetHighestScoreIndex)) (LocalVariables|GetHighestScoreIndex)))

(fn SortSaveGameData
  (while (> (Utilities|Array|Length (Variables|Default|GetSaveStruct)) 0)
    (bind (_highest_score_struct _highest_score_index) (CallFunction|DetermineHighestScoreValue))
    (Utilities|Array|Add (LocalVariables|GetTmpSaveGameStruct) _highest_score_struct)
    (Utilities|Array|RemoveIndex (Variables|Default|GetSaveStruct) _highest_score_index))
  (Variables|Default|SetSaveStruct (LocalVariables|GetTmpSaveGameStruct)))

(fn AddHighScore
  (params (New%20Score :type High%20Score%20Struct%20Structure))
  (bind _savestruct (Variables|Default|GetSaveStruct))
  (Utilities|Array|Add (Variables|Default|GetSaveStruct) New%20Score)
  (CallFunction|SortSaveGameData)
  (Utilities|Array|Resize _savestruct (Math|Integer|Min(Integer) (Utilities|Array|Length _savestruct) 4)))