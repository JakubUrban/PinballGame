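; Pinball drop target set that spells a configurable word and raises the game mode's Multiplier when all its targets are down.
; The construction script spawns one lettered BP_DropTarget child actor per uppercased character, evenly spaced by the distance between two posts, and binds its OnDrop event.
; ProcessDropTargets counts down the remaining targets, and the game mode's OnGameReset event restores the count to the word's length.
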(event Custom|ProcessDropTargets
  (bind _result (Math|Integer|DecrementInt (Variables|Default|GetTargetsCounter))
    (:%20%20
      (if (== _result 0)
        (bind _aspinball_game_mode (Utilities|Casting|CastToPinballGameMode (Game|GetGameMode)))
        (Math|Float|IncrementFloat (Variables|/Game/Blueprints/PinballGameMode.PinballGameMode_C|GetMultiplier _aspinball_game_mode))))))

(event Custom|ResetTargetsCounter
  (Variables|Default|SetTargetsCounter (Utilities|String|Len (Variables|Default|GetDropTargetText))))

(event EventBeginPlay
  (|CallParentFunction)
  (bind _aspinball_game_mode (Utilities|Casting|CastToPinballGameMode (Game|GetGameMode)))
  (EventDispatchers|BindEventtoOnGameReset _aspinball_game_mode (delegate Custom|ResetTargetsCounter)))

(event Collision|EventActorBeginOverlap
  (params (OtherActor :type Actor%20Object%20Reference))
  (|CallParentFunction OtherActor) ; This node is disabled and will not be called.\nDrag off pins to build functionality.
)

(event EventTick
  (params (DeltaSeconds :type Float%20%28single-precision%29))
  (|CallParentFunction DeltaSeconds) ; This node is disabled and will not be called.\nDrag off pins to build functionality.
)

(fn ConstructionScript
  (bind _droptargettext (Variables|Default|GetDropTargetText))
  (bind _post1 (Variables|Default|GetPost1))
  (bind _returnvalue (Class|KismetStringLibrary|ToUpper _droptargettext))
  (bind _returnvalue_2 (Utilities|String|GetCharacterArrayfromString _returnvalue))
  (|CallParentFunction)
  (for (_array_element _array_index) _returnvalue_2
    (bind _returnvalue_3 (AddComponent|AddChildActorComponent false (Math|Transform|MakeTransform (+ (* (Math|Vector|GetForwardVector _post1) (* (+ _array_index 1) (/ (Math|Vector|VectorLength (- (Variables|/Script/Engine.SceneComponent|GetRelativeLocation (Variables|Default|GetPost1)) (Variables|/Script/Engine.SceneComponent|GetRelativeLocation (Variables|Default|GetPost2)))) (Math|Conversions|ToFloat(Integer) (+ (Utilities|Array|Length _returnvalue_2) 1))))) (* (Math|Vector|GetRightVector _post1) 20)) (Variables|/Script/Engine.SceneComponent|GetRelativeRotation _post1) "1,1,1")))
    (ChildActorComponent|SetChildActorClass _returnvalue_3 "/Game/Blueprints/BP_DropTarget.BP_DropTarget_C")
    (bind _asbp_drop_target (Utilities|Casting|CastToBP_DropTarget (Variables|/Script/Engine.ChildActorComponent|GetChildActor _returnvalue_3)))
    (Rendering|Components|TextRender|SetText (Variables|/Game/Blueprints/BP_DropTarget.BP_DropTarget_C|GetTextRender _asbp_drop_target) (Utilities|Text|ToText(String) _array_element))
    (EventDispatchers|BindEventtoOnDrop _asbp_drop_target (EventDispatchers|CreateEvent :!event Custom|ProcessDropTargets))))